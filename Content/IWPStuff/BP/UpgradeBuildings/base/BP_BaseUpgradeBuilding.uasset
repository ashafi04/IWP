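; Base Blueprint for a clickable upgrade building that opens its upgrade UI when the player clicks its mesh.
; It caches the game manager on BeginPlay and uses it to reach the main UI and player manager.
; A click shows the upgrade panel and notifies the player manager.
; If that call returns false, the building swaps its own TowerUpgradeUI into the shared panel and enables custom depth rendering on its mesh.
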(event OnClicked(BuildingMesh)
  (params (TouchedComponent :type Primitive%20Component%20Object%20Reference) (ButtonPressed :type Key%20Structure :default "None"))
  (bind _game_manager_ref (Variables|Default|GetGame%20Manager%20Ref))
  (bind _main_ui_ref (Variables|/Game/IWPStuff/BP/Managers/BP_GameManager.BP_GameManager_C|GetMain%20UI%20Ref _game_manager_ref))
  (bind _bp_basetowerupgradeui (Variables|/Game/IWPStuff/UI/BP_MainUI.BP_MainUI_C|GetBP_BaseTowerUpgradeUI _main_ui_ref))
  (Widget|SetVisibility (Variables|/Game/IWPStuff/UI/BP_MainUI.BP_MainUI_C|GetUpgradeUI (Variables|/Game/IWPStuff/BP/Managers/BP_GameManager.BP_GameManager_C|GetMain%20UI%20Ref (Variables|Default|GetGame%20Manager%20Ref))) "Visible")
  (bind _same_building_selected (Default|OnUpgradeBuildingClicked (Variables|/Game/IWPStuff/BP/Managers/BP_GameManager.BP_GameManager_C|GetPlayer%20Manager%20Ref _game_manager_ref) self))
  (if (not _same_building_selected)
    (Default|RemoveCurrentUpgradeUI _bp_basetowerupgradeui)
    (Widget|Panel|AddChild (Variables|/Game/IWPStuff/UI/BP_BaseTowerUpgradeUI.BP_BaseTowerUpgradeUI_C|GetAddCustomUpgradeUIHere _bp_basetowerupgradeui) (Variables|Default|GetTower%20Upgrade%20UI))
    (Rendering|SetRenderCustomDepth (Variables|Default|GetBuilding%20Mesh) true)))

(event EventBeginPlay
  (bind _returnvalue (Actor|GetActorOfClass "/Game/IWPStuff/BP/Managers/BP_GameManager.BP_GameManager_C"))
  (Variables|Default|SetGame%20Manager%20Ref _returnvalue))

(fn ConstructionScript)