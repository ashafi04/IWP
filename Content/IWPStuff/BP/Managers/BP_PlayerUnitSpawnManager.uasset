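; BP_PlayerUnitSpawnManager tracks the player's selected lane, presumably for unit spawning, and shows which lane is active through indicator meshes.
; BeginPlay hides the static mesh component on every actor in the LaneIndicationMesh array.
; OnChangeLane hides the previous lane's indicator, stores the new index in CurrentSelectedLane and shows that lane's indicator.
; No spawning logic is present in these graphs.
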(event EventBeginPlay
  (for _array_element (Variables|Default|GetLane%20Indication%20Mesh)
    (Rendering|SetVisibility (Actor|GetComponentbyClass _array_element "/Script/Engine.StaticMeshComponent") false false)))

(event Collision|EventActorBeginOverlap
  (params (OtherActor :type Actor%20Object%20Reference)))

(event EventTick
  (params (DeltaSeconds :type Float%20%28single-precision%29)))

(fn ConstructionScript)

(fn OnChangeLane
  (params (New%20Lane%20Number :type Integer))
  (LocalVariables|SetTemp%20new%20number New%20Lane%20Number)
  (Rendering|SetVisibility (Actor|GetComponentbyClass (Utilities|Array|Get(acopy) (Variables|Default|GetLane%20Indication%20Mesh) (Variables|Default|GetCurrent%20Selected%20Lane)) "/Script/Engine.StaticMeshComponent") false false)
  (bind _output_get (Variables|Default|SetCurrent%20Selected%20Lane (LocalVariables|GetTemp%20new%20number)))
  (Rendering|SetVisibility (Actor|GetComponentbyClass (Utilities|Array|Get(acopy) (Variables|Default|GetLane%20Indication%20Mesh) _output_get) "/Script/Engine.StaticMeshComponent") true false))