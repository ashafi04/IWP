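; BP_PlayerManager sets up the player's mouse interaction and base-building UI, and switches the view between level cameras.
; On BeginPlay, Init enables cursor, click and mouse-over events, then creates the building widget with tower classes from BP_GameManager.
; Swap-left and swap-right inputs step a clamped index through the manager's cameras with blended view changes.
; Input-mapping and initial center-camera setup nodes exist in Init but are disconnected.
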(event Input|EnhancedActionEvents|EnhancedInputActionI_SwapLeft
  (params (ActionValue :type Boolean) (ElapsedSeconds :type Float%20%28double-precision%29) (TriggeredSeconds :type Float%20%28double-precision%29) (InputAction :type Input%20Action%20Object%20Reference :default "/Game/IWPStuff/Inputs/Actions/I_SwapLeft.I_SwapLeft"))
  ;[1 1 1] Swap Player to the next camera
  (:Triggered
    (bind _result (Math|Integer|DecrementInt (Variables|Default|GetCurrentCameraState))
      (:%20%20
        (if (>= _result 0)
          (Game|Player|SetViewTargetwithBlend (Variables|Default|GetPlayer%20Controller) (Utilities|Array|Get(acopy) (Variables|/Game/IWPStuff/BP/Managers/BP_GameManager.BP_GameManager_C|GetLevel%20Cameras (Variables|Default|GetGame%20Manager%20Ref)) (Variables|Default|GetCurrentCameraState)) 0.5 "VTBlend_PreBlended" 0.0 false)
          (else
            (Variables|Default|SetCurrentCameraState 0)))))))

(event Input|EnhancedActionEvents|EnhancedInputActionI_SwapRight
  (params (ActionValue :type Boolean) (ElapsedSeconds :type Float%20%28double-precision%29) (TriggeredSeconds :type Float%20%28double-precision%29) (InputAction :type Input%20Action%20Object%20Reference :default "/Game/IWPStuff/Inputs/Actions/I_SwapRight.I_SwapRight"))
  ;[1 1 1] Swap Player to the next camera
  (:Triggered
    (bind _result (Math|Integer|IncrementInt (Variables|Default|GetCurrentCameraState))
      (:%20%20
        (if (> _result 2)
          (Variables|Default|SetCurrentCameraState 2)
          (else
            (Game|Player|SetViewTargetwithBlend (Variables|Default|GetPlayer%20Controller) (Utilities|Array|Get(acopy) (Variables|/Game/IWPStuff/BP/Managers/BP_GameManager.BP_GameManager_C|GetLevel%20Cameras (Variables|Default|GetGame%20Manager%20Ref)) (Variables|Default|GetCurrentCameraState)) 0.5 "VTBlend_PreBlended" 0.0 false)))))))

(event EventBeginPlay
  (CallFunction|Init))

(event Collision|EventActorBeginOverlap
  (params (OtherActor :type Actor%20Object%20Reference)))

(event EventTick
  (params (DeltaSeconds :type Float%20%28single-precision%29)))

(fn ConstructionScript
  ;[1 1 1] Get Game Manager Ref
  (bind _returnvalue (Actor|GetActorOfClass "/Game/IWPStuff/BP/Managers/BP_GameManager.BP_GameManager_C"))
  (Variables|Default|SetGame%20Manager%20Ref _returnvalue))

(fn Init
  (bind _output_get (Variables|Default|SetPlayer%20Controller (Game|GetPlayerController 0)))
  ;[1 1 1] Enable clicking/ show cursor/ mouse over
  (Variables|/Script/Engine.PlayerController|SetbShowMouseCursor (Variables|Default|GetPlayer%20Controller) true)
  (Variables|/Script/Engine.PlayerController|SetbEnableClickEvents (Variables|Default|GetPlayer%20Controller) true)
  (Variables|/Script/Engine.PlayerController|SetbEnableMouseOverEvents (Variables|Default|GetPlayer%20Controller) true)
  ;[1 1 1] Create and display UI
  (bind _returnvalue (UserInterface|CreateWidget "/Game/IWPStuff/UI/BP_BaseBuildingWidget.BP_BaseBuildingWidget_C" (Variables|Default|GetPlayer%20Controller) (Variables|/Game/IWPStuff/BP/Managers/BP_GameManager.BP_GameManager_C|GetAll%20Tower%20Classes (Variables|Default|GetGame%20Manager%20Ref))))
  (bind _output_get_2 (Variables|Default|SetBase%20Building%20UI%20Ref _returnvalue))
  (UserInterface|Viewport|AddtoViewport _output_get_2 0))