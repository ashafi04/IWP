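; Enemy spawn manager that creates enemies targeting the castle at a random one of three spawn points.
; OnBeginEnemySpawning spawns one enemy, passes it the GameManager reference cached in the construction script and returns its score.
; SpawnDifferentEnemy randomly picks basic, armoured or flying types, limited by the GameManager's EnemyVarietyRange.
; Flying enemies spawn at a raised height and ignore collisions when spawning.
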(event Collision|EventActorBeginOverlap
  (params (OtherActor :type Actor%20Object%20Reference)))

(fn ConstructionScript
  (bind _returnvalue (Actor|GetActorOfClass "/Game/IWPStuff/BP/Managers/BP_GameManager.BP_GameManager_C"))
  (Variables|Default|SetGameManagerRef _returnvalue))

(fn OnBeginEnemySpawning
  (bind _new_enemy_spawned (CallFunction|SpawnDifferentEnemy (Math|Conversions|ToTransform(Vector) (Transformation|GetActorLocation (Utilities|Array|Get(acopy) (Variables|Default|GetEnemy%20Spawn%20Points) (Math|Random|RandomIntegerinRange 0 2)))) (Variables|Default|GetCastle)))
  (Variables|/Game/IWPStuff/BP/Units/Enemies/base/BP_BasicEnemy.BP_BasicEnemy_C|SetGame%20Manager%20Ref _new_enemy_spawned (Variables|Default|GetGameManagerRef))
  (return (Variables|/Game/IWPStuff/BP/Units/Enemies/base/BP_BasicEnemy.BP_BasicEnemy_C|GetEnemy%20Score _new_enemy_spawned)))

(fn SpawnDifferentEnemy
  (params (Spawn%20Transform :type Transform) (Castle :type Actor%20Object%20Reference))
  (LocalVariables|SetTransform Spawn%20Transform)
  (LocalVariables|SetCastle%20 Castle)
  (switch int (Math|Random|RandomIntegerinRange 0 (Variables|/Game/IWPStuff/BP/Managers/BP_GameManager.BP_GameManager_C|GetEnemy%20Variety%20Range (Variables|Default|GetGameManagerRef)))
    (:0
      (bind _returnvalue (Game|SpawnActorfromClass "/Game/IWPStuff/BP/Units/Enemies/base/BP_BasicEnemy.BP_BasicEnemy_C" (LocalVariables|GetTransform) "Undefined" 0 (LocalVariables|GetCastle%20) 0))
      (LocalVariables|SetEnemy%20Unit%20Spawned _returnvalue))
    (:1
      (bind _returnvalue_2 (Game|SpawnActorfromClass "/Game/IWPStuff/BP/Units/Enemies/ArmoredEnemy/BP_ArmouredBasicEnemy.BP_ArmouredBasicEnemy_C" (LocalVariables|GetTransform) "Undefined" 0 (LocalVariables|GetCastle%20) 0))
      (LocalVariables|SetEnemy%20Unit%20Spawned _returnvalue_2))
    (:2
      (bind _returnvalue_3 (Game|SpawnActorfromClass "/Game/IWPStuff/BP/Units/Enemies/FlyingEnemy/BP_FlyingEnemy.BP_FlyingEnemy_C" (Math|Transform|MakeTransform (Math|Vector|MakeVector (.x (.location (LocalVariables|GetTransform))) (.y (.location (LocalVariables|GetTransform))) (+ (.z (.location (LocalVariables|GetTransform))) 375.0)) (.rotation (LocalVariables|GetTransform)) (.scale (LocalVariables|GetTransform))) "AlwaysSpawn" 0 (LocalVariables|GetCastle%20) 0))
      (LocalVariables|SetEnemy%20Unit%20Spawned _returnvalue_3)))
  (return (LocalVariables|GetEnemy%20Unit%20Spawned)))