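; BP_UpgradeManager is a manager actor that holds per-class stat multipliers for Wizard and Knight units and handles purchased upgrades.
; Wizard upgrade events pass the cost to the player manager, fetched via BP_GameManager, and increment the named multiplier on success.
; SetUnitMultipliers selects the class's map and scales a unit's Attack and Defense.
; Knight upgrade events are absent, and GetUnitClassMultiplier is an unfinished stub.
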(event EventBeginPlay
  (bind _returnvalue (Actor|GetActorOfClass "/Game/IWPStuff/BP/Managers/BP_GameManager.BP_GameManager_C"))
  (Variables|Default|SetPlayer%20Manager%20Ref (Variables|/Game/IWPStuff/BP/Managers/BP_GameManager.BP_GameManager_C|GetPlayer%20Manager%20Ref _returnvalue)))

(event Collision|EventActorBeginOverlap
  (params (OtherActor :type Actor%20Object%20Reference)))

(event EventTick
  (params (DeltaSeconds :type Float%20%28single-precision%29)))

(event EventUpgradeWizardDamage
  (params (Stat%20Name :type String) (Upgrade%20Cost :type Integer))
  (Variables|Default|SetUpgraded%20Stat%20Name Stat%20Name)
  (bind _can_purchase (Default|OnSingleUpgradeClicked (Variables|Default|GetPlayer%20Manager%20Ref) Upgrade%20Cost))
  (if _can_purchase
    (Utilities|Map|Add (Variables|Default|GetWizard%20Unit%20Multipliers) (Variables|Default|GetUpgraded%20Stat%20Name) (+ (.Value (Utilities|Map|Find (Variables|Default|GetWizard%20Unit%20Multipliers) (Variables|Default|GetUpgraded%20Stat%20Name))) 1))))

(event EventUpgradeWizardDefense
  (params (Stat%20name :type String) (Upgrade%20Cost :type Integer))
  (bind _upgradepurchased (CallFunction|CheckCanPurchaseUpgrade Stat%20name Upgrade%20Cost))
  (if _upgradepurchased
    (Utilities|Map|Add (Variables|Default|GetWizard%20Unit%20Multipliers) (Variables|Default|GetUpgraded%20Stat%20Name) (+ (.Value (Utilities|Map|Find (Variables|Default|GetWizard%20Unit%20Multipliers) (Variables|Default|GetUpgraded%20Stat%20Name))) 1))))

(fn ConstructionScript)

(fn GetUnitClassMultiplier
  (params (Unit%20Class%20Name :type String))
  (LocalVariables|SetClass%20name%20 Unit%20Class%20Name)
  (for _array_element (LocalVariables|GetUnit%20Class%20Ref)
    (if (Utilities|Enum|Equal(Enum) (LocalVariables|GetClass%20name%20) (.UnitClass (Utilities|GetClassDefaults _array_element)))
      _)))

(fn SetUnitMultipliers
  (params (Unit%20 :type Player%20Base%20Unit%20Object%20Reference))
  (bind _output_get (LocalVariables|Settemp%20unit%20ref Unit%20))
  (switch string (Variables|/Script/IWP.PlayerBaseUnit|GetUnitClass _output_get)
    (:Default
      (Development|PrintString "SET MULTIPLIER FAILED"))
    (:Wizard
      (LocalVariables|SetSelection%20index 0)
      (Variables|/Script/IWP.BaseUnit|SetAttack (LocalVariables|Gettemp%20unit%20ref) (* (.Value (Utilities|Map|Find (Utilities|Select :Index (LocalVariables|GetSelection%20index) :Option%200 (Variables|Default|GetWizard%20Unit%20Multipliers) :Option%201 (Variables|Default|GetKnight%20Unit%20Multipliers)) "Damage")) (Variables|/Script/IWP.BaseUnit|GetAttack (LocalVariables|Gettemp%20unit%20ref))) :!label _label)
      (Variables|/Script/IWP.BaseUnit|SetDefense (LocalVariables|Gettemp%20unit%20ref) (* (.Value (Utilities|Map|Find (Utilities|Select :Index (LocalVariables|GetSelection%20index) :Option%200 (Variables|Default|GetWizard%20Unit%20Multipliers) :Option%201 (Variables|Default|GetKnight%20Unit%20Multipliers)) "Defense")) (Variables|/Script/IWP.BaseUnit|GetDefense (LocalVariables|Gettemp%20unit%20ref)))))
    (:Knight
      (LocalVariables|SetSelection%20index 1)
      (goto _label))))

(fn CheckCanPurchaseUpgrade
  (params (Stat%20 :type String) (Cost :type Integer))
  (Variables|Default|SetUpgraded%20Stat%20Name Stat%20)
  (bind _can_purchase (Default|OnSingleUpgradeClicked (Variables|Default|GetPlayer%20Manager%20Ref) Cost))
  (return _can_purchase))