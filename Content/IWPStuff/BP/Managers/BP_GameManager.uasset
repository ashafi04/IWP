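; Game manager that sets up the main UI and player manager, and holds the stat multipliers for units.
; Init creates the UI with the tower classes and spawns the player manager, whose gold total Tick pushes to the UI.
; Wizard damage upgrades raise their multiplier after the player manager approves the cost, while the defense upgrade is empty.
; The construction script also creates a UI, and the castle-overlap game-over check is disconnected.
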(event Custom|CheckGameEnd
  ;[1 1 1] Check if any enemy has reached target points in base
)

(event EventBeginPlay
  (CallFunction|Init))

(event EventUpgradeWizardDefense)

(event EventTick
  (params (DeltaSeconds :type Float%20%28single-precision%29))
  (Rendering|Components|TextRender|SetText (Variables|/Game/IWPStuff/UI/BP_MainUI.BP_MainUI_C|GetTotalGoldAmount (Variables|Default|GetManager%20UI%20Ref)) (Utilities|Text|ToText(Integer) (Variables|/Game/IWPStuff/BP/Managers/BP_PlayerManager.BP_PlayerManager_C|GetTotal%20Gold%20Amount%20 (Variables|Default|GetPlayer%20Manager%20Ref)))))

(event EventUpgradeWizardDamage
  (params (Stat%20Name :type String) (Upgrade%20Cost :type Integer))
  (bind _unit_multipliers (Variables|Default|GetUnit%20Multipliers))
  (bind _value (Utilities|Map|Find _unit_multipliers Stat%20Name))
  ;[1 1 1] Increase Wizard Damage By 1 every upgrade
  (bind _can_purchase (Default|OnSingleUpgradeClicked (Variables|Default|GetPlayer%20Manager%20Ref) Upgrade%20Cost))
  (if _can_purchase
    (Utilities|Map|Add (Variables|Default|GetUnit%20Multipliers) Stat%20Name (+ _value 1))
    (Development|PrintString "UPGRADE DAMAGE")
    (Development|PrintString (Utilities|String|ToString(Integer) _value))))

(fn ConstructionScript
  (bind _returnvalue (Game|ConstructObjectfromClass "/Game/IWPStuff/UI/BP_MainUI.BP_MainUI_C" (Variables|Default|GetAll%20Tower%20Classes)))
  (UserInterface|Viewport|AddtoViewport _returnvalue 0)
  (Variables|Default|SetManager%20UI%20Ref _returnvalue))

(fn Init
  ;[1 1 1] Create and set UI ref
  (bind _returnvalue (UserInterface|CreateWidget "/Game/IWPStuff/UI/BP_MainUI.BP_MainUI_C" 0 (Variables|Default|GetAll%20Tower%20Classes)))
  (UserInterface|Viewport|AddtoViewport _returnvalue 0)
  (Variables|Default|SetManager%20UI%20Ref _returnvalue)
  (bind _returnvalue_2 (Game|SpawnActorfromClass "/Game/IWPStuff/BP/Managers/BP_PlayerManager.BP_PlayerManager_C" (Math|Transform|MakeTransform "0, 0, 0") "Undefined" 0 0 0))
  (Variables|Default|SetPlayer%20Manager%20Ref _returnvalue_2))

(fn GetUnitMultiplier
  (params (Stat :type String))
  (return (.Value (Utilities|Map|Find (Variables|Default|GetUnit%20Multipliers) Stat))))