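; Base tower projectile that damages enemies on overlap, meant as a parent for projectile variants.
; Mesh overlaps skip sphere components (tower range collision) and act only on BP_BasicEnemy actors tagged Enemy.
; A hit calls the empty ProjectileEffect hook for child classes, spawns particles, subtracts the owning tower's Damage from enemy Health and destroys the projectile.
; If Health reaches zero or below, it flags EnemyDead on UnitRef.
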(event OnComponentBeginOverlap(ProjectileMesh)
  (params (OverlappedComponent :type Primitive%20Component%20Object%20Reference) (OtherActor :type Actor%20Object%20Reference) (OtherComp :type Primitive%20Component%20Object%20Reference) (OtherBodyIndex :type Integer) (bFromSweep :type Boolean) (SweepResult :type Hit%20Result%20Structure%20%28by%20ref%29))
  (if (not (== (Utilities|GetClass OtherComp) "/Script/Engine.SphereComponent"))
    (if (Actor|ActorHasTag OtherActor "Enemy")
      (bind _asbp_basic_enemy (Utilities|Casting|CastToBP_BasicEnemy OtherActor))
      (CallFunction|ProjectileEffect _asbp_basic_enemy)
      ;[1 1 1] Spawn particles when projectile hits an enemy
      (Effects|SpawnEmitteratLocation (Variables|Default|GetDeathParticles) (Transformation|GetActorLocation self))
      (bind _output_get (Variables|/Script/IWP.BaseUnit|SetHealth _asbp_basic_enemy (- (Variables|/Script/IWP.BaseUnit|GetHealth _asbp_basic_enemy) (Variables|/Game/IWPStuff/BP/Towers/Base/BP_BasicTower.BP_BasicTower_C|GetDamage (Variables|/Game/IWPStuff/BP/Towers/Base/BP_BasicTowerUnit.BP_BasicTowerUnit_C|GetTower%20Owner%20Ref (Variables|Default|GetUnit%20Ref))))))
      (Actor|DestroyActor)
      (if (<= _output_get 0)
        (Variables|/Game/IWPStuff/BP/Towers/Base/BP_BasicTowerUnit.BP_BasicTowerUnit_C|SetEnemy%20Dead (Variables|Default|GetUnit%20Ref) true)))))

(event EventBeginPlay)

(event EventTick
  (params (DeltaSeconds :type Float%20%28single-precision%29)))

(fn ConstructionScript)

(fn ProjectileEffect
  (params (Enemy%20Hit :type BP%20Basic%20Enemy%20Object%20Reference))
  ;[1 1 1] Function to be used in child classes
)