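; Actor component that makes its owner clickable, toggling an outline mesh on and off with each click.
; On BeginPlay it binds to the owner's OnClicked event and caches the first StaticMeshComponent tagged "Outline".
; Each click flips the IsClicked flag and, if that mesh is valid, sets its visibility to match.
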(event Custom|OnMouseClicked
  (params (TouchedActor :type Actor%20Object%20Reference) (ButtonPressed :type Key%20Structure :default "None"))
  (Variables|Default|SetIsClicked (not (Variables|Default|GetIsClicked)))
  (Utilities|IsValid (Variables|Default|GetStatic%20Mesh%20Ref)
    (:Is%20Valid
      (Rendering|SetVisibility (Variables|Default|GetStatic%20Mesh%20Ref) (Variables|Default|GetIsClicked) false))))

(event EventBeginPlay
  (bind _returnvalue (Components|GetOwner))
  (bind _returnvalue_2 (Actor|GetComponentsbyTag _returnvalue "/Script/Engine.StaticMeshComponent" "Outline"))
  (bind _output (Utilities|Array|Get(acopy) _returnvalue_2))
  (EventDispatchers|BindEventtoOnClicked _returnvalue (delegate Custom|OnMouseClicked))
  (Utilities|IsValid _output
    (:Is%20Valid
      (Variables|Default|SetStatic%20Mesh%20Ref _output))))

(event EventTick
  (params (DeltaSeconds :type Float%20%28single-precision%29)))