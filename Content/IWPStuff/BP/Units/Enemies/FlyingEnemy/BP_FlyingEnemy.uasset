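; Flying enemy Blueprint that heads for the castle target through its AI controller when play begins.
; On death, a one-time sequence raises fly speed, sets a Y-axis plane constraint normal and redirects movement to a point below the castle target.
; After a short delay it gives the player gold, destroys itself and increments the GameManager kill count.
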(event OnComponentBeginOverlap(Vision)
  (params (OverlappedComponent :type Primitive%20Component%20Object%20Reference) (OtherActor :type Actor%20Object%20Reference) (OtherComp :type Primitive%20Component%20Object%20Reference) (OtherBodyIndex :type Integer) (bFromSweep :type Boolean) (SweepResult :type Hit%20Result%20Structure%20%28by%20ref%29)))

(event EventBeginPlay
  (|CallParentFunction)
  (AI|Navigation|MovetoLocation (AI|GetAIController self) (Transformation|GetActorLocation (Variables|Default|GetCastleTarget)) 1.0 true true false true 0))

(event EventOnDeath
  (bind _castletarget (Variables|Default|GetCastleTarget))
  (bind _charactermovement (Variables|Character|GetCharacterMovement))
  (bind _returnvalue (Transformation|GetActorLocation _castletarget))
  (Utilities|FlowControl|DoOnce false
    (:Completed
      (Variables|/Script/Engine.CharacterMovementComponent|SetMaxFlySpeed _charactermovement 1e+03)
      (Class|MovementComponent|SetPlaneConstraintNormal _charactermovement "0.000000,1.000000,0.000000")
      (AI|Navigation|MovetoLocation (AI|GetAIController self) (Math|Vector|MakeVector (.x _returnvalue) (.y _returnvalue) (- (.z _returnvalue) 1e+02)) 1.0 true true false true 0)
      (Utilities|FlowControl|Delay 0.7)
      (CallFunction|GiveGoldtoPlayer)
      (Actor|DestroyActor)
      (Math|Integer|IncrementInt (Variables|/Game/IWPStuff/BP/Managers/BP_GameManager.BP_GameManager_C|GetTotal%20Enemies%20Killed%20 (Variables|Default|GetGame%20Manager%20Ref))))))

(fn ConstructionScript
  (|CallParentFunction))