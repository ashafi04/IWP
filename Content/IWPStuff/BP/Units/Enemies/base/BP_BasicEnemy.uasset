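; Base enemy unit that marches toward a castle target and fights allied units it meets along the way.
; Vision overlaps set the target: allies switch it to attack, other units make it wait until that target leaves.
; Attacks run from Tick on a countdown scaled by AttackSpeed but not delta time, playing goblin animation and stab sound.
; When the target becomes invalid, it resumes walking to the castle.
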(event OnComponentBeginOverlap(Vision)
  (params (OverlappedComponent :type Primitive%20Component%20Object%20Reference) (OtherActor :type Actor%20Object%20Reference) (OtherComp :type Primitive%20Component%20Object%20Reference) (OtherBodyIndex :type Integer) (bFromSweep :type Boolean) (SweepResult :type Hit%20Result%20Structure%20%28by%20ref%29))
  (if (not (Components|ComponentHasTag OtherComp "Vision"))
    (bind _asbase_unit (Utilities|Casting|CastToBaseUnit OtherActor))
    (bind _output_get (Variables|Default|SetTargetUnit _asbase_unit))
    (if (Variables|/Script/IWP.BaseUnit|GetIsAlly _output_get)
      (Class|NavMovementComponent|StopActiveMovement (Variables|Character|GetCharacterMovement))
      (Variables|Default|SetMovementStateEnum "ATTACK")
      (else
        (CallFunction|OnWait)))))

(event OnComponentEndOverlap(Vision)
  (params (OverlappedComponent :type Primitive%20Component%20Object%20Reference) (OtherActor :type Actor%20Object%20Reference) (OtherComp :type Primitive%20Component%20Object%20Reference) (OtherBodyIndex :type Integer))
  (if (and (== (Variables|Default|GetMovementStateEnum) 0) (== OtherActor (Variables|Default|GetTargetUnit)))
    (AI|Navigation|SimpleMovetoActor (Pawn|GetController) (Variables|Default|GetCastleTarget))))

(event EventBeginPlay
  (AI|Navigation|SimpleMovetoActor (Pawn|GetController) (Variables|Default|GetCastleTarget)))

(event EventOnDeath)

(event EventTick
  (params (DeltaSeconds :type Float%20%28single-precision%29))
  (if (== (Variables|Default|GetMovementStateEnum) 2)
    (Utilities|IsValid (Variables|Default|GetTargetUnit)
      (:Is%20Valid
        (CallFunction|OnAttack))
      (:Is%20Not%20Valid
        (Variables|Default|SetMovementStateEnum "WALK")
        (AI|AIMoveTo self "0, 0, 0" (Variables|Default|GetCastleTarget) 5.0 false)))))

(fn ConstructionScript)

(fn OnAttack
  (bind _audio (Variables|Default|GetAudio))
  ;[1 1 1] Check if enemy can attack
  (bind _output_get (Variables|Default|SetAttack%20Countdown%20Timer (- (Variables|Default|GetAttack%20Countdown%20Timer) (* 1 (Variables|Default|GetAttackSpeed)))))
  (if (<= _output_get 0.0)
    (Components|Animation|PlayAnimation (Variables|Character|GetMesh) "/Game/Goblin/Animation/Anim_Goblin_body_attack.Anim_Goblin_body_attack" true)
    (Audio|Components|Audio|SetSound _audio "/Game/IWPStuff/Audio/Weapons/stab1.stab1")
    (Audio|Components|Audio|Play _audio 0.0)
    (Class|BaseUnit|TakeDamage (Variables|Default|GetTargetUnit) self)
    (Variables|Default|SetAttack%20Countdown%20Timer (Variables|Default|GetAttackTimer))))

(fn OnWait
  (Variables|Default|SetMovementStateEnum "IDLE")
  (Class|NavMovementComponent|StopActiveMovement (Variables|Character|GetCharacterMovement)))