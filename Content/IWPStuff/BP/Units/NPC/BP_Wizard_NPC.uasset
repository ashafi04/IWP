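; BP_Wizard_NPC is a wizard NPC that wanders between randomly picked actors from PointArray.
; It starts an AI MoveTo on BeginPlay, picks another point on each success, and sets MovementEnum to WALK while moving.
; Each Tick has a one-in-ten chance to call Stop, which halts movement and sets IDLE, then resume wandering after a short Delay.
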(event Custom|Move%20to%20Random%20Point
  (AI|AIMoveTo self "0, 0, 0" (.OutItem (Utilities|Array|Random (Variables|Default|Getpoint%20Array))) 1.0 false
    (:then
      (Variables|Default|SetMovement%20Enum "WALK"))
    (:OnSuccess
      (CallFunction|MovetoRandomPoint))))

(event EventBeginPlay
  (CallFunction|MovetoRandomPoint))

(event EventTick
  (params (DeltaSeconds :type Float%20%28single-precision%29))
  (if (== (Math|Random|RandomIntegerinRange 0 9) 1)
    (CallFunction|Stop)
    (Utilities|FlowControl|Delay 3.0)
    (CallFunction|MovetoRandomPoint)))

(fn ConstructionScript)

(fn Stop
  (Class|NavMovementComponent|StopActiveMovement (Variables|Character|GetCharacterMovement))
  (Variables|Default|SetMovement%20Enum "IDLE"))