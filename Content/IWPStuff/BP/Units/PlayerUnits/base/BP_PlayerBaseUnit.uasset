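; Base Blueprint for player units, reacting to other units that enter its Vision component and handling its own death.
; On overlap it ignores components tagged Vision and stores any BaseUnit as TargetUnit, then loops the attack animation if that unit is flagged IsAlly, otherwise stops active movement.
; Tick prints Health every frame, and OnDeath prints a message and destroys the actor.
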(event OnComponentBeginOverlap(Vision)
  (params (OverlappedComponent :type Primitive%20Component%20Object%20Reference) (OtherActor :type Actor%20Object%20Reference) (OtherComp :type Primitive%20Component%20Object%20Reference) (OtherBodyIndex :type Integer) (bFromSweep :type Boolean) (SweepResult :type Hit%20Result%20Structure%20%28by%20ref%29))
  (if (not (Components|ComponentHasTag OtherComp "Vision"))
    (bind _asbase_unit (Utilities|Casting|CastToBaseUnit OtherActor))
    (bind _output_get (Variables|Default|SetTargetUnit _asbase_unit))
    (if (Variables|/Script/IWP.BaseUnit|GetIsAlly _output_get)
      (Components|Animation|PlayAnimation (Variables|Character|GetMesh) "/Game/BattleWizardPolyart/Animations/Attack01Anim.Attack01Anim" true)
      (else
        (Class|NavMovementComponent|StopActiveMovement (Variables|Character|GetCharacterMovement))))))

(event EventBeginPlay)

(event EventTick
  (params (DeltaSeconds :type Float%20%28single-precision%29))
  (Development|PrintString (Utilities|String|ToString(Integer) (Variables|Default|GetHealth))))

(event EventOnDeath
  (Development|PrintString "DIED")
  (Actor|DestroyActor))

(fn ConstructionScript)