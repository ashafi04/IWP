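; BP_BasicTower is a tower Blueprint that tracks enemies in range, with unfinished target selection.
; Sphere overlap adds Enemy-tagged BasicEnemy actors implementing UnitInteractionInterface to EnemyTargets, but nothing removes them.
; A looping timer calls Retarget when CurrentTarget is invalid, as does the current target leaving the sphere.
; Retarget does nothing: its closest-enemy loop is disconnected and never updates the shortest distance.
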(event OnComponentEndOverlap(Sphere)
  (params (OverlappedComponent :type Primitive%20Component%20Object%20Reference) (OtherActor :type Actor%20Object%20Reference) (OtherComp :type Primitive%20Component%20Object%20Reference) (OtherBodyIndex :type Integer))
  ;[1 1 1] Retarget when current target is dead or out of range
  (if (== OtherActor (Variables|Default|GetCurrentTarget))
    (CallFunction|Retarget false)))

(event OnComponentBeginOverlap(Sphere)
  (params (OverlappedComponent :type Primitive%20Component%20Object%20Reference) (OtherActor :type Actor%20Object%20Reference) (OtherComp :type Primitive%20Component%20Object%20Reference) (OtherBodyIndex :type Integer) (bFromSweep :type Boolean) (SweepResult :type Hit%20Result%20Structure%20%28by%20ref%29))
  ;[1 1 1] Check if pawn that is in range implements interface and is an enemy
  (if (and (Utilities|DoesObjectImplementInterface OtherActor "/Game/IWPStuff/BP/Interfaces/UnitInteractionInterface.UnitInteractionInterface_C") (Actor|ActorHasTag OtherActor "Enemy"))
    (bind _asbasic_enemy (Utilities|Casting|CastToBasicEnemy OtherActor))
    (Utilities|Array|AddUnique (Variables|Default|GetEnemyTargets) _asbasic_enemy)))

(event Custom|OnRetargetEnemy
  ;[1 1 1] Retarget when current target is dead or out of range
  (Utilities|IsValid (Variables|Default|GetCurrentTarget)
    (:Is%20Not%20Valid
      (CallFunction|Retarget true))))

(event EventBeginPlay
  (bind _returnvalue (Utilities|Time|SetTimerbyEvent (delegate Custom|OnRetargetEnemy) 0.5 true))
  (Variables|Default|SetTimer%20handle _returnvalue))

(fn ConstructionScript)

(fn Retarget
  (params (Target%20Destroyed :type Boolean))
  (if Target%20Destroyed
    _))