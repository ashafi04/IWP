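; BP_IceTowerUnit is the ice tower's shooting unit, which fires ice projectiles at its target.
; Each tick, once it can shoot and has rotated, it spawns a scaled-down BP_IceProjectile at its spawn point, passing itself as reference, then clears CanShoot.
; If the valid target has no health left, it asks the owning tower to retarget to the nearest enemy.
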(event EventTick
  (params (DeltaSeconds :type Float%20%28single-precision%29))
  (bind _projectile_spawn_location (Variables|Default|GetProjectile%20Spawn%20Location))
  (bind _unit_s_target (Variables|Default|GetUnit's%20Target))
  (bind _returnvalue (Transformation|GetWorldTransform _projectile_spawn_location))
  (|CallParentFunction DeltaSeconds)
  (if (and (Variables|Default|GetCan%20Shoot) (Variables|Default|GetHas%20Rotated))
    (Utilities|IsValid _unit_s_target
      (:Is%20Valid
        (if (> (Variables|/Script/IWP.BaseUnit|GetHealth _unit_s_target) 0)
          (Game|SpawnActorfromClass "/Game/IWPStuff/BP/Projectiles/BP_IceProjectile.BP_IceProjectile_C" (Math|Transform|MakeTransform (.location _returnvalue) (.rotation _returnvalue) "0.350000,0.350000,0.350000") "AlwaysSpawn" 0 self 0)
          (Variables|Default|SetCan%20Shoot false)
          (else
            (Default|RetargettoNearestEnemytoTower (Variables|Default|GetTower%20Owner%20Ref))))))))

(fn ConstructionScript
  (|CallParentFunction))