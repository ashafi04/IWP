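; Base tower actor that the player places with the cursor and that then targets nearby enemies.
; Until placed, a looping timer moves it to the cursor trace hit and tints it green or red by the surface's Buildable tag; left-click restores materials and activates it.
; Once active, sphere overlaps collect enemies, ignoring Vision components.
; Overlap and death events retarget to the nearest enemy, which Tick passes to TowerUnitRef.
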(event OnComponentEndOverlap(Sphere)
  (params (OverlappedComponent :type Primitive%20Component%20Object%20Reference) (OtherActor :type Actor%20Object%20Reference) (OtherComp :type Primitive%20Component%20Object%20Reference) (OtherBodyIndex :type Integer))
  ;[1 1 1] Retarget when current target is out of range
  (if (not (Components|ComponentHasTag OtherComp "Vision"))
    (if (== OtherActor (Variables|Default|GetCurrentTarget))
      (CallFunction|RetargettoNearestEnemytoTower))))

(event OnComponentBeginOverlap(Tower)
  (params (OverlappedComponent :type Primitive%20Component%20Object%20Reference) (OtherActor :type Actor%20Object%20Reference) (OtherComp :type Primitive%20Component%20Object%20Reference) (OtherBodyIndex :type Integer) (bFromSweep :type Boolean) (SweepResult :type Hit%20Result%20Structure%20%28by%20ref%29)))

(event OnComponentBeginOverlap(Sphere)
  (params (OverlappedComponent :type Primitive%20Component%20Object%20Reference) (OtherActor :type Actor%20Object%20Reference) (OtherComp :type Primitive%20Component%20Object%20Reference) (OtherBodyIndex :type Integer) (bFromSweep :type Boolean) (SweepResult :type Hit%20Result%20Structure%20%28by%20ref%29))
  ;[1 1 1] Dont add when enemy vision enters into Tower Range
  (if (Variables|Default|GetisActive)
    (if (not (Components|ComponentHasTag OtherComp "Vision"))
      ;[1 1 1] Check if pawn that is in range implements interface and is an enemy
      (if (and (Utilities|DoesObjectImplementInterface OtherActor "/Game/IWPStuff/BP/Interfaces/UnitInteractionInterface.UnitInteractionInterface_C") (Actor|ActorHasTag OtherActor "Enemy"))
        (bind _asbasic_enemy (Utilities|Casting|CastToBasicEnemy OtherActor))
        (bind _returnvalue (Utilities|Array|AddUnique (Variables|Default|GetEnemyTargets) _asbasic_enemy))
        ;[1 1 1] Retarget when first enemy is in range
        (if (== _returnvalue 0)
          (CallFunction|RetargettoNearestEnemytoTower))))))

(event Custom|OnPlaceBuilding
  (CallFunction|SetMeshMaterials)
  (Variables|Default|SetisActive true)
  (Utilities|Time|ClearandInvalidateTimerbyHandle (stale EventBeginPlay _returnvalue)))

(event Custom|Check%20Actor%20Placement
  (bind _can_place (CallFunction|CheckActorCollisions))
  (CallFunction|SetPlacementMaterial _can_place))

(event EventBeginPlay
  ;[1 1 1] On actor spawned, save mesh materials and set mesh to use green/red material for placement
  (Variables|Default|SetTower%20Mesh%20Materials (Rendering|Material|GetMaterials (Variables|Default|GetTower)))
  (CallFunction|SetPlacementMaterial false)
  (bind _returnvalue (Utilities|Time|SetTimerbyEvent (delegate Custom|Check%20Actor%20Placement) 0.01 true)))

(event EventTick
  (params (DeltaSeconds :type Float%20%28single-precision%29))
  (if (Variables|Default|GetisActive)
    ;[1 1 1] Update Tower Unit Target once tower is active
    (CallFunction|UpdateUnitTargeting)))

(event EventOnEnemyDeath
  ;[1 1 1] When enemy dies. remove from array and retarget
  (Utilities|Array|RemoveItem (Variables|Default|GetEnemyTargets) (Variables|Default|GetCurrentTarget))
  (CallFunction|RetargettoNearestEnemytoTower))

(event MouseInput|EventActorOnClicked
  (params (ButtonPressed :type Key%20Structure :default "None"))
  ;[1 1 1] do Checks and place tower on cursor
  (if (== ButtonPressed "LeftMouseButton")
    (if (not (Variables|Default|GetisActive))
      (if (not (Variables|Default|GetisRedPlacement))
        (CallFunction|OnPlaceBuilding)))))

(fn ConstructionScript)

(fn RetargettoNearestEnemytoTower
  (bind _enemytargets (Variables|Default|GetEnemyTargets))
  (bind _defaultsceneroot (Variables|Default|GetDefaultSceneRoot))
  (bind _returnvalue (Transformation|GetWorldLocation _defaultsceneroot))
  (bind (_distance _returnvalue_2) (Actor|FindNearestActor _returnvalue _enemytargets))
  ;[1 1 1] Find nearest Enemy to the tower
  ;[1 1 1] Check if
  (if (Utilities|Array|IsNotEmpty _enemytargets)
    ;[1 1 1] Set new target to
    (Variables|Default|SetDist%20To%20Nearest%20Enemy _distance)
    (bind _asbasic_enemy (Utilities|Casting|CastToBasicEnemy _returnvalue_2))
    (Variables|Default|SetCurrentTarget _asbasic_enemy)))

(fn SetMeshMaterials
  (for (_array_element _array_index) (Variables|Default|GetTower%20Mesh%20Materials)
    (Rendering|Material|SetMaterial (Variables|Default|GetTower) _array_index _array_element)))

(fn UpdateUnitTargeting
  (if (!= (Variables|Default|GetCurrentTarget) (Variables|/Game/IWPStuff/BP/Towers/Base/BP_BasicTowerUnit.BP_BasicTowerUnit_C|GetTarget (Variables|Default|GetTower%20Unit%20Ref)))
    (Variables|/Game/IWPStuff/BP/Towers/Base/BP_BasicTowerUnit.BP_BasicTowerUnit_C|SetTarget (Variables|Default|GetTower%20Unit%20Ref) (Variables|Default|GetCurrentTarget))))

(fn SetPlacementMaterial
  (params (Can%20Place%20Tower :type Boolean))
  (bind _output_get (Variables|Default|SetisRedPlacement (not Can%20Place%20Tower)))
  (if _output_get
    (LocalVariables|SetTemp%20Material (LocalVariables|GetRed))
    (else
      (LocalVariables|SetTemp%20Material (LocalVariables|GetGreen))))
  (for _index (range 0 (Utilities|Array|LastIndex (Variables|Default|GetTower%20Mesh%20Materials)))
    (Rendering|Material|SetMaterial (Variables|Default|GetTower) _index (LocalVariables|GetTemp%20Material)))
  (Variables|Default|SetisActive false))

(fn CheckActorCollisions
  (bind _returnvalue (Game|GetPlayerController 0))
  (bind _hitresult (Game|Player|GetHitResultUnderCursorbyChannel _returnvalue "TraceTypeQuery1" true))
  (bind (_bblockinghit _binitialoverlap _time _distance _location _impactpoint _normal _impactnormal _physmat _hitactor) (Collision|BreakHitResult _hitresult))
  (Utilities|IsValid _hitactor
    (:Is%20Valid
      (LocalVariables|SetTemp%20Actor%20Hit _hitactor)
      (if (!= (LocalVariables|GetTemp%20Actor%20Hit) self)
        (Transformation|SetActorLocation _location false false)
        (Variables|Default|SetActor%20Instigator (LocalVariables|GetTemp%20Actor%20Hit) :!label _label)
        (else
          (Utilities|IsValid (Variables|Default|GetActor%20Instigator)
            (:Is%20Valid
              _)
            (:Is%20Not%20Valid
              (goto _label)))))
      (return (Actor|ActorHasTag (Variables|Default|GetActor%20Instigator) "Buildable")))))