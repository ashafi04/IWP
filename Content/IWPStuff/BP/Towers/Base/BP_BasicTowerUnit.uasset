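; Base tower unit that aims at its assigned target and tracks when it is ready to shoot.
; A looping timer interpolates actor yaw toward the target and applies pitch to the projectile spawn point.
; Tick advances reload by a fixed per-frame step, making it frame-rate dependent, and relays enemy deaths to the owning tower.
; CheckCanShoot sets CanShoot once reload completes with a valid target; no firing happens here.
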(event Custom|OnRotate
  (bind _returnvalue (Transformation|GetActorLocation))
  (bind _returnvalue_2 (Utilities|Time|GetWorldDeltaSeconds))
  (bind _returnvalue_3 (Transformation|GetActorRotation))
  (bind _unit_s_target (Variables|Default|GetUnit's%20Target))
  (bind _returnvalue_4 (Transformation|GetActorLocation _unit_s_target))
  (bind _returnvalue_5 (Math|Rotator|FindLookatRotation _returnvalue _returnvalue_4))
  (bind _returnvalue_6 (Math|Interpolation|RInterpTo _returnvalue_3 _returnvalue_5 _returnvalue_2 1e+02))
  ;[1 1 1] Rotate Unit to face Target
  (Variables|Default|SetHas%20Rotated false)
  (Utilities|IsValid _unit_s_target
    (:Is%20Valid
      (bind _returnvalue_7 (Transformation|SetActorRotation (Math|Rotator|MakeRotator 0.0 0.0 (.yaw _returnvalue_6))))
      (Transformation|SetRelativeRotation (Variables|Default|GetProjectile%20Spawn%20Location) (Math|Rotator|MakeRotator 0.0 (.pitch _returnvalue_6) 0.0) false false)
      (Variables|Default|SetHas%20Rotated _returnvalue_7))))

(event EventBeginPlay
  (Utilities|Time|SetTimerbyEvent (delegate Custom|OnRotate) 0.04 true))

(event EventTick
  (params (DeltaSeconds :type Float%20%28single-precision%29))
  (bind _tower_owner_ref (Variables|Default|GetTower%20Owner%20Ref))
  (Variables|Default|SetTemp%20Reload%20Time (+ (Variables|Default|GetTemp%20Reload%20Time) 0.08))
  (if (Variables|Default|GetEnemy%20Dead)
    (Utilities|IsValid _tower_owner_ref
      (:Is%20Valid
        (Default|OnEnemyDeath _tower_owner_ref)
        (Variables|Default|SetEnemy%20Dead false))))
  (CallFunction|CheckCanShoot))

(fn ConstructionScript)

(fn CheckCanShoot
  (if (>= (Variables|Default|GetTemp%20Reload%20Time) (Variables|Default|GetMax%20Reload%20Time))
    (Utilities|IsValid (Variables|Default|GetUnit's%20Target)
      (:Is%20Valid
        (Variables|Default|SetCan%20Shoot true)
        (Variables|Default|SetTemp%20Reload%20Time 0.0))
      (:Is%20Not%20Valid
        (Variables|Default|SetCan%20Shoot false)))))