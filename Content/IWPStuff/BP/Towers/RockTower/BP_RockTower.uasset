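; BP_RockTower is a clickable tower actor that spawns and owns a single rock tower unit.
; When clicked while active, it spawns a BP_RockTowerUnit at the SPAWNUNITHERE component's location if its unit reference is not valid.
; The unit receives the tower as its owner, and the tower stores the unit reference.
; Click, tick and construction all call the parent class's logic.
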(event MouseInput|EventActorOnClicked
  (params (ButtonPressed :type Key%20Structure :default "None"))
  (|CallParentFunction ButtonPressed)
  (if (Variables|Default|GetisActive)
    (Utilities|IsValid (Variables|Default|GetTower%20Unit%20Ref)
      (:Is%20Not%20Valid
        ;[1 1 1] Spawn Unit when Tower is placed and set references
        (bind _returnvalue (Game|SpawnActorfromClass "/Game/IWPStuff/BP/Towers/RockTower/BP_RockTowerUnit.BP_RockTowerUnit_C" (Math|Conversions|ToTransform(Vector) (Transformation|GetWorldLocation (Variables|Default|GetSPAWN%20UNIT%20HERE))) "AlwaysSpawn" 0 self 0))
        (Variables|Default|SetTower%20Unit%20Ref _returnvalue)))))

(event EventTick
  (params (DeltaSeconds :type Float%20%28single-precision%29))
  (|CallParentFunction 0.0))

(fn ConstructionScript
  (|CallParentFunction))