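; BP_RockTowerUnit is the unit of the rock tower that fires rock projectiles at its target.
; It relies on its parent class Tick and fires only when CanShoot and HasRotated are set and the target is valid.
; A living target triggers a scaled-down BP_RockProjectile spawn at ProjectileSpawnLocation, passing itself as UnitRef, then clears CanShoot.
; A target without health makes the owning tower retarget to its nearest enemy.
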(event EventBeginPlay)

(event EventTick
  (params (DeltaSeconds :type Float%20%28single-precision%29))
  (bind _projectile_spawn_location (Variables|Default|GetProjectile%20Spawn%20Location))
  (bind _unit_s_target (Variables|Default|GetUnit's%20Target))
  (bind _returnvalue (Transformation|GetWorldTransform _projectile_spawn_location))
  ;[1 1 1] Check from base class if unit can shoot
  (|CallParentFunction 0.0)
  (if (and (Variables|Default|GetCan%20Shoot) (Variables|Default|GetHas%20Rotated))
    (Utilities|IsValid _unit_s_target
      (:Is%20Valid
        (if (> (Variables|/Script/IWP.BaseUnit|GetHealth _unit_s_target) 0)
          ;[1 1 1] Spawn Projectile and reset Can Shoot var
          (Game|SpawnActorfromClass "/Game/IWPStuff/BP/Projectiles/BP_RockProjectile.BP_RockProjectile_C" (Math|Transform|MakeTransform (.location _returnvalue) (.rotation _returnvalue) "0.200000,0.200000,0.200000") "AlwaysSpawn" 0 self 0)
          (Variables|Default|SetCan%20Shoot false)
          (else
            (Default|RetargettoNearestEnemytoTower (Variables|Default|GetTower%20Owner%20Ref))))))))

(fn ConstructionScript)